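; BP_CoinBox is a coin box actor whose FeedCoinEvent turns its mesh into a growing cube.
; The event swaps in the Cube mesh and basic shape material, plays Timeline_Big to drive relative scale, then sets box collision to query-only.
; The Construction Script sets the initial material from MyMat through MatToMat.
; The sphere overlap event is empty, and the debug prints are disconnected, one noted as required to avoid a bug.
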(event OnComponentBeginOverlap(SphereComp)
  (params (OverlappedComponent :type Primitive%20Component%20Object%20Reference) (OtherActor :type Actor%20Object%20Reference) (OtherComp :type Primitive%20Component%20Object%20Reference) (OtherBodyIndex :type Integer) (bFromSweep :type Boolean) (SweepResult :type Hit%20Result%20Structure%20%28by%20ref%29)))

(event EventBeginPlay)

(event Collision|EventActorBeginOverlap
  (params (OtherActor :type Actor%20Object%20Reference)))

(event EventTick
  (params (DeltaSeconds :type Float%20%28single-precision%29)))

(event EventFeedCoinEvent
  (bind _meshcomp (Variables|Default|GetMeshComp))
  (Components|StaticMesh|SetStaticMesh _meshcomp "/Game/StaticMesh/Cube.Cube")
  (Rendering|Material|SetMaterial _meshcomp 0 "/Game/Material/BasicShapeMaterial.BasicShapeMaterial")
  (bind _155 (Timeline|Timeline_Big PlayFromStart)
    (:Update
      (Transformation|SetRelativeScale3D (Variables|Default|GetMeshComp) (Math|Conversions|ToVector(Float) _155)))
    (:Finished
      (Collision|SetCollisionEnabled (Variables|Default|GetBoxComp) "QueryOnly"))))

(fn ConstructionScript
  (Rendering|Material|SetMaterial (Variables|Default|GetMeshComp) 0 (CallFunction|MattoMat (Variables|Default|GetMyMat))))